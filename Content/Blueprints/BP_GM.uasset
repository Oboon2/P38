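; BP_GM, apparently a game mode by its name, tracks the actors tagged "Target" and reports a clear once none remain.
; It gathers the tagged actors and their count at BeginPlay, then repeats the world search every Tick.
; While the count is zero, it prints "Clear!" each frame.
; An OpenLevelByName node with level "None" is left unconnected, so no level change occurs.
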(event EventBeginPlay
  (bind _outactors (Actor|GetAllActorswithTag "Target"))
  (bind _output_get (Variables|Default|SetTarget _outactors))
  (Variables|Default|SetTotalCount (Utilities|Array|Length _output_get)))

(event EventTick
  (params (DeltaSeconds :type Float%20%28single-precision%29))
  (bind _outactors (Actor|GetAllActorswithTag "Target"))
  (bind _output_get (Variables|Default|SetTarget _outactors))
  (bind _output_get_2 (Variables|Default|SetTotalCount (Utilities|Array|Length _output_get)))
  (if (== _output_get_2 0)
    (Development|PrintString "Clear!")))

(fn ConstructionScript)