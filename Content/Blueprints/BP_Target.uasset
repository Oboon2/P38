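; BP_Target is a target actor that constantly rotates and dissolves away when it takes any damage.
; BeginPlay creates a dynamic material instance on the static mesh.
; AnyDamage plays a timeline that drives the material's Cut parameter.
; The Delay and DestroyActor hang off the timeline's Update pin, so destruction follows one second after the first update, independent of timeline completion.
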(event EventBeginPlay
  (bind _returnvalue (Rendering|Material|CreateDynamicMaterialInstance (Variables|Default|GetStaticMesh) 0 0 "None" :!class /Script/Engine.PrimitiveComponent))
  (Variables|Default|SetDissolveMaterial _returnvalue))

(event Collision|EventActorBeginOverlap
  (params (OtherActor :type Actor%20Object%20Reference)))

(event EventTick
  (params (DeltaSeconds :type Float%20%28single-precision%29))
  (Transformation|AddActorLocalRotation "1.000000,1.000000,1.000000" false false))

(event Game|Damage|EventAnyDamage
  (params (Damage :type Float%20%28single-precision%29) (DamageType :type Damage%20Type%20Object%20Reference) (InstigatedBy :type Controller%20Object%20Reference) (DamageCauser :type Actor%20Object%20Reference))
  (bind _새_트랙_0 (Timeline|타임라인_0 Play)
    (:Update
      (Rendering|Material|SetScalarParameterValue (Variables|Default|GetDissolveMaterial) "Cut" _새_트랙_0 :!class /Script/Engine.MaterialInstanceDynamic)
      (Utilities|FlowControl|Delay 1.0)
      (Actor|DestroyActor))))

(fn ConstructionScript)