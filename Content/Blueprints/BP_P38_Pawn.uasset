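; Player-controlled P-38 plane pawn that flies, steers and fires rockets.
; Tick applies constant forward movement input and spins both propellers through NewFunction0.
; Roll and Pitch axes apply frame-rate-scaled local rotation, both using RollSpeed.
; Fire spawns BP_Rocket at the Arrow; HomingFire also makes the rocket home on the mesh of the first "Target"-tagged actor, if it is a BP_Target.
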(event EventBeginPlay)

(event Collision|EventActorBeginOverlap
  (params (OtherActor :type Actor%20Object%20Reference)))

(event EventTick
  (params (DeltaSeconds :type Float%20%28single-precision%29))
  (Utilities|FlowControl|Sequence
    (:then_0
      (Pawn|Input|AddMovementInput (* (Transformation|GetActorForwardVector) 0.3) 1.0 false))
    (:then_1
      (CallFunction|NewFunction0 (Variables|Default|GetPropeller1)))
    (:then_2
      (CallFunction|NewFunction0 (Variables|Default|GetPropeller2)))))

(event Input|ActionEvents|InputActionFire
  (params (Key :type Key%20Structure))
  (:Pressed
    (Game|SpawnActorfromClass "/Game/Blueprints/BP_Rocket.BP_Rocket_C" (Transformation|GetWorldTransform (Variables|Default|GetArrow)) "Undefined" 0 0)))

(event Input|ActionEvents|InputActionHomingFire
  (params (Key :type Key%20Structure))
  (:Pressed
    (bind _returnvalue (Game|SpawnActorfromClass "/Game/Blueprints/BP_Rocket.BP_Rocket_C" (Transformation|GetWorldTransform (Variables|Default|GetArrow)) "Undefined" 0 0))
    (Variables|Default|SetLaunchedRocket _returnvalue)
    (Variables|/Script/Engine.ProjectileMovementComponent|SetbIsHomingProjectile (Variables|/Game/Blueprints/BP_Rocket.BP_Rocket_C|GetProjectileMovement (Variables|Default|GetLaunchedRocket)) true)
    (Variables|/Script/Engine.ProjectileMovementComponent|SetMaxSpeed (Variables|/Game/Blueprints/BP_Rocket.BP_Rocket_C|GetProjectileMovement (Variables|Default|GetLaunchedRocket)) 5e+03)
    (Variables|/Script/Engine.ProjectileMovementComponent|SetHomingAccelerationMagnitude (Variables|/Game/Blueprints/BP_Rocket.BP_Rocket_C|GetProjectileMovement (Variables|Default|GetLaunchedRocket)) 2e+04)
    (bind _outactors (Actor|GetAllActorswithTag "Target"))
    (bind _asbp_target (Utilities|Casting|CastToBP_Target (Utilities|Array|Get(acopy) _outactors)))
    (Variables|/Script/Engine.ProjectileMovementComponent|SetHomingTargetComponent (Variables|/Game/Blueprints/BP_Rocket.BP_Rocket_C|GetProjectileMovement (Variables|Default|GetLaunchedRocket)) (Variables|/Game/Blueprints/BP_Target.BP_Target_C|GetStaticMesh _asbp_target))))

(event Input|AxisEvents|InputAxisPitch
  (params (AxisValue :type Float%20%28single-precision%29))
  (Transformation|AddActorLocalRotation (Math|Rotator|MakeRotator 0.0 (* (Input|AxisValues|GetPitch) (Variables|Default|GetRollSpeed) (Utilities|Time|GetWorldDeltaSeconds)) 0.0) false false))

(event Input|AxisEvents|InputAxisRoll
  (params (AxisValue :type Float%20%28single-precision%29))
  (Transformation|AddActorLocalRotation (Math|Rotator|MakeRotator (* (Input|AxisValues|GetRoll) (Variables|Default|GetRollSpeed) (Utilities|Time|GetWorldDeltaSeconds)) 0.0 0.0) false false))

(fn ConstructionScript)

(fn NewFunction0
  (params (self2 :type Scene%20Component%20Object%20Reference))
  (Transformation|AddLocalRotation self2 (Math|Rotator|MakeRotator (* (Variables|Default|GetPropellerRotateSpeed) (Utilities|Time|GetWorldDeltaSeconds)) 0.0 0.0) false false))