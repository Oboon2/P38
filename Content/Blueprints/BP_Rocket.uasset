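; Rocket projectile actor that explodes and deals damage when it overlaps another actor.
; BeginPlay sets a limited lifespan so stray rockets clean themselves up.
; On overlap it ignores actors tagged Rocket or Player; otherwise it destroys itself, plays an explosion sound and particle effect, and applies fixed damage to the hit actor.
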(event EventBeginPlay
  (Actor|SetLifeSpan 5.0))

(event Collision|EventActorBeginOverlap
  (params (OtherActor :type Actor%20Object%20Reference))
  (Variables|Default|SetOtherActor OtherActor)
  (if (not (Actor|ActorHasTag (Variables|Default|GetOtherActor) "Rocket"))
    (if (not (Actor|ActorHasTag (Variables|Default|GetOtherActor) "Player"))
      (Actor|DestroyActor)
      (Audio|SpawnSoundatLocation "/Game/StarterContent/Audio/Explosion_Cue.Explosion_Cue" (Transformation|GetActorLocation) "0, 0, 0" 1.0 1.0 0.0 0 0)
      (Effects|SpawnEmitteratLocation "/Game/StarterContent/Particles/P_Explosion.P_Explosion" (Transformation|GetActorLocation) (Transformation|GetActorRotation))
      (Game|Damage|ApplyDamage (Variables|Default|GetOtherActor) 3e+01 0 0))))

(event EventTick
  (params (DeltaSeconds :type Float%20%28single-precision%29)))

(fn ConstructionScript)